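; Functional test that drives the player's car through a short scripted movement sequence.
; A SetUp event stores the Player, whose CarMoveComponent StartTest feeds with timed vertical and horizontal inputs separated by delays.
; The car moves with both inputs positive, then reverses vertical input with horizontal zeroed, then stops.
; The test always finishes as Succeeded, with no check on the resulting movement.
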(event Custom|Set%20Up
  (params (Player :type BP%20Test%20Car%20Object%20Reference))
  (Variables|Default|SetPlayer Player))

(event EventPrepareTest)

(event EventStartTest
  (bind _player (Variables|Default|GetPlayer))
  (bind _returnvalue (Actor|GetComponentbyClass _player "/Script/ProductionEnv.CarMoveComponent"))
  (Class|CarMoveComponent|MoveVertical _returnvalue 1.0)
  (Class|CarMoveComponent|MoveHorizontal _returnvalue 1.0)
  (Utilities|FlowControl|Delay 0.5)
  (Class|CarMoveComponent|MoveVertical _returnvalue -1.0)
  (Class|CarMoveComponent|MoveHorizontal _returnvalue 0.0)
  (Utilities|FlowControl|Delay 1.0)
  (Class|CarMoveComponent|MoveVertical _returnvalue 0.0)
  (Class|FunctionalTest|FinishTest "Succeeded" "Moved the car"))

(fn ConstructionScript)